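; BP_EnemySpot is an actor that spawns enemy BP_Card actors at a fixed set of spawn point components.
; BeginPlay gathers the six spawn points into a Slots array.
; SpawnEnemies waits briefly, then places each requested card at a random slot and removes that slot, printing a message when none is left.
; Every card gets the same hardcoded "Hero Of Light" data and is flagged as an enemy card.
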(event Custom|SpawnEnemies
  (params (NoToSpawn :type Integer))
  (Utilities|FlowControl|Delay 1.666)
  (for _index (range 0 (- NoToSpawn 1))
    (bind _output_get (Variables|Default|SetSelectedPount (.OutItem (Utilities|Array|Random (Variables|Default|GetSlots)))))
    (Utilities|IsValid _output_get
      (:Is%20Valid
        (Game|SpawnActorfromClass "/Game/Blueprints/BP_Card.BP_Card_C" (Math|Transform|MakeTransform (Transformation|GetWorldLocation (Variables|Default|GetSelectedPount)) "0, 0, 0" "1.000000,1.000000,1.000000") "Undefined" "MultiplyWithRoot" 0 (Utilities|Struct|Makestru_CArd "Hero Of Light" 0 "(INVALID)" (Utilities|Map|MakeMap "NewEnumerator5" 2) 1 0 false "" 0 false "NewEnumerator0" false false 0 0) true 0 0)
        (Utilities|Array|RemoveItem (Variables|Default|GetSlots) (Variables|Default|GetSelectedPount)))
      (:Is%20Not%20Valid
        (Development|PrintString "No slot to spawn")))))

(event EventBeginPlay
  (Variables|Default|SetSlots (Utilities|Array|MakeArray (Variables|Default|GetComp_SpawnpointScene1) (Variables|Default|GetComp_SpawnpointScene2) (Variables|Default|GetComp_SpawnpointScene3) (Variables|Default|GetComp_SpawnpointScene4) (Variables|Default|GetComp_SpawnpointScene5) (Variables|Default|GetComp_SpawnpointScene6))))

(fn ConstructionScript)