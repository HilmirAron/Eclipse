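; BP_TapIcon is a clickable resource icon for an assigned card, destroying itself at BeginPlay without one.
; MyNumber picks its type from the card's resource keys, setting the texture on dynamic materials for icon and hover highlight.
; Clicking forwards enemy icons to the card; otherwise Wood, Iron and Food increment BP_GameCamera totals, stop battle and consume the icon.
; Magic and War feed active battles through UIFightBar, while Gold has no click handling.
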(event OnBeginCursorOver(Icon)
  (params (TouchedComponent :type Primitive%20Component%20Object%20Reference))
  (Rendering|SetVisibility (Variables|Default|GetIconHighlight) true false))

(event OnEndCursorOver(Icon)
  (params (TouchedComponent :type Primitive%20Component%20Object%20Reference))
  (Rendering|SetVisibility (Variables|Default|GetIconHighlight) false false))

(event OnClicked(Icon)
  (params (TouchedComponent :type Primitive%20Component%20Object%20Reference) (ButtonPressed :type Key%20Structure :default "None"))
  (if (Variables|Default|GetIsEnemy)
    (Default|ClickOther (Variables|Default|GetAssignedCard))
    (else
      (bind _asbp_game_camera (Utilities|Casting|CastToBP_GameCamera (Game|Player|GetPlayerPawn 0)))
      (switch Utilities|FlowControl|Switch|Switchonenum_Resources (Variables|Default|GetMyType)
        (:NewEnumerator0
          (Math|Integer|IncrementInt (Variables|/Game/Blueprints/BP_GameCamera.BP_GameCamera_C|GetWood _asbp_game_camera)
            (:%20%20
              (Default|StopBattle (Variables|/Game/UI/UI_GameMain.UI_GameMain_C|GetUI_FightBar (Variables|/Game/Blueprints/BP_GameCamera.BP_GameCamera_C|GetMainUIRef _asbp_game_camera)) :!label _label)
              (Actor|DestroyActor))))
        (:NewEnumerator1
          (Math|Integer|IncrementInt (Variables|/Game/Blueprints/BP_GameCamera.BP_GameCamera_C|GetSteel _asbp_game_camera)
            (:%20%20
              (goto _label))))
        (:NewEnumerator2
          (Math|Integer|IncrementInt (Variables|/Game/Blueprints/BP_GameCamera.BP_GameCamera_C|GetFood _asbp_game_camera)
            (:%20%20
              (goto _label))))
        (:NewEnumerator4
          (if (Variables|/Game/UI/UI_FightBar.UI_FightBar_C|GetBattleIsOn (Variables|/Game/UI/UI_GameMain.UI_GameMain_C|GetUI_FightBar (Variables|/Game/Blueprints/BP_GameCamera.BP_GameCamera_C|GetMainUIRef _asbp_game_camera)))
            (Default|AddBattleIcon (Variables|/Game/UI/UI_GameMain.UI_GameMain_C|GetUI_FightBar (Variables|/Game/Blueprints/BP_GameCamera.BP_GameCamera_C|GetMainUIRef _asbp_game_camera)) "NewEnumerator4")))
        (:NewEnumerator5
          (if (Variables|/Game/UI/UI_FightBar.UI_FightBar_C|GetBattleIsOn (Variables|/Game/UI/UI_GameMain.UI_GameMain_C|GetUI_FightBar (Variables|/Game/Blueprints/BP_GameCamera.BP_GameCamera_C|GetMainUIRef _asbp_game_camera)))
            (Default|AddBattleIcon (Variables|/Game/UI/UI_GameMain.UI_GameMain_C|GetUI_FightBar (Variables|/Game/Blueprints/BP_GameCamera.BP_GameCamera_C|GetMainUIRef _asbp_game_camera)) "NewEnumerator5")))))))

(event EventBeginPlay
  (bind _assignedcard (Variables|Default|GetAssignedCard))
  (Utilities|IsValid _assignedcard
    (:Is%20Valid
      (bind _keys (Utilities|Map|Keys (.resources (Variables|/Game/Blueprints/BP_Card.BP_Card_C|GetMyData _assignedcard))))
      (Variables|Default|SetMyType (Utilities|Array|Get(acopy) _keys (Variables|Default|GetMyNumber)))
      (bind _returnvalue (Rendering|Material|CreateDynamicMaterialInstance (Variables|Default|GetIcon) 0 0 "None" :!class /Script/Engine.PrimitiveComponent))
      (Rendering|Material|SetTextureParameterValue _returnvalue "Icon" (Utilities|Select :Index (Variables|Default|GetMyType) :NewEnumerator0 "/Game/Images/T_TimburIcon.T_TimburIcon" :NewEnumerator1 "/Game/Images/T_IronIcon.T_IronIcon" :NewEnumerator2 "/Game/Images/T_FoodIcon.T_FoodIcon" :NewEnumerator3 "/Game/Images/t_CoinIcon.t_CoinIcon" :NewEnumerator4 "/Game/Images/T_MagicIcon.T_MagicIcon" :NewEnumerator5 "/Game/Images/T_WarIcon.T_WarIcon"))
      (bind _returnvalue_2 (Rendering|Material|CreateDynamicMaterialInstance (Variables|Default|GetIconHighlight) 0 0 "None" :!class /Script/Engine.PrimitiveComponent))
      (Rendering|Material|SetTextureParameterValue _returnvalue_2 "Icon" (Utilities|Select :Index (Variables|Default|GetMyType) :NewEnumerator0 "/Game/Images/T_TimburIcon.T_TimburIcon" :NewEnumerator1 "/Game/Images/T_IronIcon.T_IronIcon" :NewEnumerator2 "/Game/Images/T_FoodIcon.T_FoodIcon" :NewEnumerator3 "/Game/Images/t_CoinIcon.t_CoinIcon" :NewEnumerator4 "/Game/Images/T_MagicIcon.T_MagicIcon" :NewEnumerator5 "/Game/Images/T_WarIcon.T_WarIcon")))
    (:Is%20Not%20Valid
      (Actor|DestroyActor))))

(fn ConstructionScript)