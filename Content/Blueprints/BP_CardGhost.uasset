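; BP_CardGhost is a ghost actor for a card, apparently a preview with an optional area-of-effect indicator.
; On BeginPlay it creates a dynamic material on its static mesh and destroys the Area component when its card data has no area effect.
; A MaterialChange event switches that material's Color parameter between red and neutral grey according to a boolean.
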(event Custom|MaterialChange
  (params (Red :type Boolean))
  (if Red
    (Rendering|Material|SetVectorParameterValue (Variables|Default|GetMaterialRef) "Color" "(R=1.000000,G=0.016830,B=0.000000,A=1.000000)" :!class /Script/Engine.MaterialInstanceDynamic)
    (else
      (Rendering|Material|SetVectorParameterValue (Variables|Default|GetMaterialRef) "Color" "(R=0.603922,G=0.603922,B=0.603922,A=1.000000)" :!class /Script/Engine.MaterialInstanceDynamic))))

(event EventBeginPlay
  (bind _returnvalue (Rendering|Material|CreateDynamicMaterialInstance (Variables|Default|GetStaticMesh) 0 0 "None" :!class /Script/Engine.PrimitiveComponent))
  (Variables|Default|SetMaterialRef _returnvalue)
  (if (not (.hasareaeffect (Variables|Default|Getdata)))
    (Components|DestroyComponent (Variables|Default|Getarea))))

(fn ConstructionScript)