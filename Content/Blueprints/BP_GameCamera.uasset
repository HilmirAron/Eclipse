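; BP_GameCamera acts as the card game's central manager, creating the main UI and tracking days, resources, domination points and the deck.
; New days damage cards and periodically spawn enemies, while new turns restore player card icons and clear resources.
; Domination thresholds raise the deck level, rebuilding a shuffled deck from the card data table and showing level-up or win screens.
; It also handles mouse-positioned card previews and debug-prints the deck every tick.
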(event Custom|NewDay
  (bind _result (Math|Integer|IncrementInt (Variables|Default|GetDay))
    (:%20%20
      (if (== _result (Variables|Default|GetNextEnemyPlay))
        (Variables|Default|SetNextEnemyPlay (+ (Variables|Default|GetNextEnemyPlay) 9))
        (Default|SpawnEnemies (Variables|Default|GetEnemyBoardRef) 2))
      (bind _outactors (Actor|GetAllActorsOfClass "/Game/Blueprints/BP_Card.BP_Card_C"))
      (for _array_element _outactors
        (Default|DealDamage _array_element)))))

(event Custom|PreviewCArd
  (params (MyData :type Stru%20C%20Ard%20Structure) (AssignedCard :type BP%20Card%20Object%20Reference))
  (Variables|Default|SetHoldPreview false)
  (Utilities|IsValid (Variables|Default|GetCurrentPreview)
    (:Is%20Valid
      (Widget|RemovefromParent (Variables|Default|GetCurrentPreview)))
    (:Is%20Not%20Valid
      _))
  (bind _returnvalue (UserInterface|CreateWidget "/Game/UI/UI_card.UI_card_C" 0 MyData true true AssignedCard))
  (bind _returnvalue_2 (Class|WidgetLayoutLibrary|GetMousePositiononViewport))
  (UserInterface|Viewport|AddtoViewport _returnvalue 0)
  (Class|UserWidget|SetPositioninViewport _returnvalue (+ _returnvalue_2 "(X=50.000000,Y=-125.000000)") true)
  (Variables|Default|SetCurrentPreview _returnvalue))

(event Custom|StopPreview
  (if (not (Variables|Default|GetHoldPreview))
    (Utilities|IsValid (Variables|Default|GetCurrentPreview)
      (:Is%20Valid
        (Widget|RemovefromParent (Variables|Default|GetCurrentPreview))
        (Variables|Default|SetCurrentPreview 0)))))

(event Custom|NewTurn
  (bind _outactors (Actor|GetAllActorsOfClass "/Game/Blueprints/BP_Card.BP_Card_C"))
  (for _array_element _outactors
    (if (not (Variables|/Game/Blueprints/BP_Card.BP_Card_C|GetIsEnemyCard _array_element))
      (Default|RestoreIcons _array_element true "NewEnumerator0")))
  (Variables|Default|SetWood 0)
  (Variables|Default|SetSteel 0)
  (Variables|Default|SetFood 0))

(event Custom|AddDominationPoints
  (params (add :type Integer))
  (bind _output_get (Variables|Default|SetDominationPoint (+ (Variables|Default|GetDominationPoint) add)))
  (if (>= _output_get (Utilities|Select :Index (Variables|Default|GetDeckLevel) :Option%200 0 :Option%201 1500 :Option%202 5500 :Option%203 15000))
    (bind _result (Math|Integer|IncrementInt (Variables|Default|GetDeckLevel))
      (:%20%20
        (CallFunction|ReSetDeck)
        (if (> _result 3)
          (bind _returnvalue (UserInterface|CreateWidget "/Game/UI/UI_Win.UI_Win_C"))
          (UserInterface|Viewport|AddtoViewport _returnvalue 0)
          (else
            (bind _returnvalue_2 (UserInterface|CreateWidget "/Game/UI/UI_DeckLevelUp.UI_DeckLevelUp_C"))
            (UserInterface|Viewport|AddtoViewport _returnvalue_2 0)))))))

(event EventBeginPlay
  (bind _returnvalue (Game|GetPlayerController 0))
  (bind _returnvalue_2 (UserInterface|CreateWidget "/Game/UI/UI_GameMain.UI_GameMain_C" 0 self))
  (UserInterface|Viewport|AddtoViewport _returnvalue_2 0)
  (Variables|Default|SetMainUIRef _returnvalue_2)
  (Variables|/Script/Engine.PlayerController|SetbShowMouseCursor _returnvalue true)
  (Variables|/Script/Engine.PlayerController|SetbEnableMouseOverEvents _returnvalue true)
  (Variables|/Script/Engine.PlayerController|SetbEnableClickEvents _returnvalue true)
  (CallFunction|ReSetDeck))

(event EventTick
  (params (DeltaSeconds :type Float%20%28single-precision%29))
  (for _array_element (Variables|Default|GetDeckContent)
    (Development|PrintString (Utilities|String|ToString(Name) _array_element) true true "(R=1.000000,G=0.272382,B=0.000000,A=1.000000)" 0.01)))

(fn ConstructionScript)

(fn GetAllWarIcons
  (bind _outactors (Actor|GetAllActorsOfClass "/Game/Blueprints/BP_TapIcon.BP_TapIcon_C"))
  (for _array_element _outactors
    (if (not (Variables|/Game/Blueprints/BP_TapIcon.BP_TapIcon_C|GetIsEnemy _array_element))
      (if (Utilities|Select :Index (Variables|/Game/Blueprints/BP_TapIcon.BP_TapIcon_C|GetMyType _array_element) :NewEnumerator0 false :NewEnumerator1 false :NewEnumerator2 false :NewEnumerator3 false :NewEnumerator4 false :NewEnumerator5 true :NewEnumerator6 false)
        (Utilities|Array|Add (LocalVariables|GettempIcons) _array_element))))
  (return (LocalVariables|GettempIcons)))

(fn ReSetDeck
  (Utilities|Array|Clear (Variables|Default|GetDeckContent))
  (bind _outrownames (DataTable|GetDataTableRowNames "/Game/data_CArds.data_CArds"))
  (for _array_element _outrownames
    (bind _returnvalue (Utilities|GetDataTableRow "/Game/data_CArds.data_CArds" _array_element)
      (:then
        (if (<= (.level _returnvalue) (Variables|Default|GetDeckLevel))
          (for _index (range 0 (.ammount _returnvalue))
            (Utilities|Array|Add (Variables|Default|GetDeckContent) _array_element))))))
  (Utilities|Array|Shuffle (Variables|Default|GetDeckContent)))