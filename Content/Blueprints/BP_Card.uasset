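; Board card actor for a card game: animates onto the table, shows MyData through a widget, and serves both player and enemy cards.
; Quick-play cards grant resources, fire effects and vanish; others spawn attached BP_TapIcons, tracking removed ones for restoration.
; Clicking drags allies through a Tick gate or starts battle with enemies, whose attacks scale with icon count.
; Instant, end-of-turn, death and active effects are hardcoded switches on card name.
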(event OnBeginCursorOver(Widget)
  (params (TouchedComponent :type Primitive%20Component%20Object%20Reference))
  ;[1 1 1] Preview and stop preview
  (Default|PreviewCArd (Variables|Default|GetPlayerREf) (Variables|Default|GetMyData) self))

(event OnReleased(Widget)
  (params (TouchedComponent :type Primitive%20Component%20Object%20Reference) (ButtonReleased :type Key%20Structure :default "None"))
  ;[1 1 1] If you hit ally card, you begin dragging or maybe show card to activate effects maybe.
  (Utilities|FlowControl|Gate true) ; enters at Close
)

(event OnClicked(Widget)
  (params (TouchedComponent :type Primitive%20Component%20Object%20Reference) (ButtonPressed :type Key%20Structure :default "None"))
  (if (Variables|Default|GetIsEnemyCard)
    ;[1 0 0] If you click on enemy card. Battle starts.
    (Default|StopBattle (Variables|/Game/UI/UI_GameMain.UI_GameMain_C|GetUI_FightBar (Variables|/Game/Blueprints/BP_GameCamera.BP_GameCamera_C|GetMainUIRef (Variables|Default|GetPlayerREf))) false)
    (Default|BeginBattle (Variables|/Game/UI/UI_GameMain.UI_GameMain_C|GetUI_FightBar (Variables|/Game/Blueprints/BP_GameCamera.BP_GameCamera_C|GetMainUIRef (Variables|Default|GetPlayerREf))) (Variables|Default|GetMyData) self)
    (else
      ;[1 1 1] If you hit ally card, you begin dragging or maybe show card to activate effects maybe.
      (Default|StopBattle (Variables|/Game/UI/UI_GameMain.UI_GameMain_C|GetUI_FightBar (Variables|/Game/Blueprints/BP_GameCamera.BP_GameCamera_C|GetMainUIRef (Variables|Default|GetPlayerREf))) false)
      (Variables|/Game/Blueprints/BP_GameCamera.BP_GameCamera_C|SetHoldPreview (Variables|Default|GetPlayerREf) true)
      (Utilities|FlowControl|Gate true) ; enters at Open
    )))

(event OnEndCursorOver(Widget)
  (params (TouchedComponent :type Primitive%20Component%20Object%20Reference))
  ;[1 1 1] Preview and stop preview
  (Default|StopPreview (Variables|Default|GetPlayerREf)))

(event Custom|OnPlayed
  (bind _mydata (Variables|Default|GetMyData))
  (if (.quickplay (Variables|Default|GetMyData))
    ;[1 0.4847 0.7226] QuickPlay Logic
    ;;[1 1 1] Slowly flies up
    (bind _newtrack_0 (Timeline|FlyOut Play)
      (:Update
        (Transformation|SetRelativeLocation (Variables|Default|GetCArdBody) (Math|Vector|Lerp(Vector) "0, 0, 0" "0.000000,0.000000,5.000000" _newtrack_0) false false))
      (:Finished
        (bind _asbp_game_camera (Utilities|Casting|CastToBP_GameCamera (Game|Player|GetPlayerPawn 0)))
        ;;[1 1 1] Adds the right resource and then goes away
        (bind _keys (Utilities|Map|Keys (.resources _mydata)))
        (for _array_element _keys
          (switch Utilities|FlowControl|Switch|Switchonenum_Resources _array_element
            (:NewEnumerator0
              (Variables|/Game/Blueprints/BP_GameCamera.BP_GameCamera_C|SetWood _asbp_game_camera (+ (Variables|/Game/Blueprints/BP_GameCamera.BP_GameCamera_C|GetWood _asbp_game_camera) (.Value (Utilities|Map|Find (.resources _mydata) _array_element)))))
            (:NewEnumerator1
              (Variables|/Game/Blueprints/BP_GameCamera.BP_GameCamera_C|SetSteel _asbp_game_camera (+ (Variables|/Game/Blueprints/BP_GameCamera.BP_GameCamera_C|GetSteel _asbp_game_camera) (.Value (Utilities|Map|Find (.resources _mydata) _array_element)))))
            (:NewEnumerator2
              (Variables|/Game/Blueprints/BP_GameCamera.BP_GameCamera_C|SetFood _asbp_game_camera (+ (Variables|/Game/Blueprints/BP_GameCamera.BP_GameCamera_C|GetFood _asbp_game_camera) (.Value (Utilities|Map|Find (.resources _mydata) _array_element)))))
            (:NewEnumerator3
              (Variables|/Game/Blueprints/BP_GameCamera.BP_GameCamera_C|SetGold _asbp_game_camera (+ (Variables|/Game/Blueprints/BP_GameCamera.BP_GameCamera_C|GetGold _asbp_game_camera) (.Value (Utilities|Map|Find (.resources _mydata) _array_element)))))))
        (CallFunction|CustomEffect) ; CustomEffect for those who do more than add icons
        (Actor|DestroyActor)))
    (else
      (CallFunction|AddFloatingIcons))))

(event Custom|AddFloatingIcons
  (bind _mydata (Variables|Default|GetMyData))
  ;[1 1 1] Add icons
  (bind _keys (Utilities|Map|Keys (.resources _mydata)))
  (for _array_element _keys
    (for _index (range 0 (- (.Value (Utilities|Map|Find (.resources _mydata) _array_element)) 1))
      (bind _returnvalue (Game|SpawnActorfromClass "/Game/Blueprints/BP_TapIcon.BP_TapIcon_C" (Math|Transform|MakeTransform (Math|Vector|MakeVector 0.0 0.0 0.0) "0, 0, 0" "1.000000,1.000000,1.000000") "Undefined" "MultiplyWithRoot" 0 self 0 _array_element (Variables|Default|GetIsEnemyCard) 0))
      (Utilities|Array|Add (Variables|Default|GetIcons) _returnvalue)
      (Transformation|AttachActorToActor _returnvalue self "None" "KeepWorld" "KeepWorld" "KeepWorld" true)))
  ;;[1 1 1] Set their location
  (CallFunction|ReorderIcons))

(event Custom|RemoveIcon
  (params (Icon :type BP%20Tap%20Icon%20Object%20Reference) (Temporarly :type Boolean))
  ;[1 1 1] Cleanly remove icons
  (if Temporarly
    _
    (else
      (Utilities|Array|RemoveItem (Variables|Default|GetIcons) Icon)
      (Utilities|Array|Add (Variables|Default|GetMissingIcons) (Variables|/Game/Blueprints/BP_TapIcon.BP_TapIcon_C|GetMyType Icon))))
  (Actor|DestroyActor Icon))

(event Custom|RestoreIcons
  (params (AllIcons :type Boolean) (Types :type Array%20of%20enum_Resources%20Enums :default "NewEnumerator0"))
  (bind _removefrommissing (Variables|Default|GetREmoveFromMissing))
  (bind _missingicons (Variables|Default|GetMissingIcons))
  (if AllIcons
    (for _array_element (Variables|Default|GetMissingIcons)
      (if (not (or (Utilities|Enum|Equal(Enum) _array_element "NewEnumerator5") (Utilities|Enum|Equal(Enum) _array_element "NewEnumerator4"))) ; Do not restore War and Magic Icons On Turn start
        (bind _returnvalue (Game|SpawnActorfromClass "/Game/Blueprints/BP_TapIcon.BP_TapIcon_C" (Math|Transform|MakeTransform (Math|Vector|MakeVector 0.0 0.0 0.0) "0, 0, 0" "1.000000,1.000000,1.000000") "Undefined" "MultiplyWithRoot" 0 self 0 _array_element false 0))
        (Utilities|Array|Add (Variables|Default|GetIcons) _returnvalue)
        (Transformation|AttachActorToActor _returnvalue self "None" "KeepWorld" "KeepWorld" "KeepWorld" true)
        (Utilities|Array|Add (Variables|Default|GetREmoveFromMissing) _array_element)))
    (CallFunction|ReorderIcons)
    (for _array_element_2 _removefrommissing
      (Utilities|Array|RemoveItem (Variables|Default|GetMissingIcons) _array_element_2))
    (Utilities|Array|Clear _removefrommissing)
    (else
      (for _array_element_3 Types
        (if (Utilities|Array|ContainsItem (Variables|Default|GetMissingIcons) _array_element_3)
          (bind _returnvalue_2 (Game|SpawnActorfromClass "/Game/Blueprints/BP_TapIcon.BP_TapIcon_C" (Math|Transform|MakeTransform (Math|Vector|MakeVector 0.0 0.0 0.0) "0, 0, 0" "1.000000,1.000000,1.000000") "Undefined" "MultiplyWithRoot" 0 self 0 _array_element_3 false 0))
          (Utilities|Array|Add (Variables|Default|GetIcons) _returnvalue_2)
          (Transformation|AttachActorToActor _returnvalue_2 self "None" "KeepWorld" "KeepWorld" "KeepWorld" true)
          (Utilities|Array|Add (Variables|Default|GetREmoveFromMissing) _array_element_3)))
      (CallFunction|ReorderIcons)
      (for _array_element_4 (Variables|Default|GetREmoveFromMissing)
        (Utilities|Array|RemoveIndex _missingicons (Utilities|Array|FindItem _missingicons _array_element_4))))))

(event Custom|DealDamage
  (bind _playerref (Variables|Default|GetPlayerREf))
  ;[1 0 0] Make Enemy Deal damage
  (if (Variables|Default|GetIsEnemyCard)
    (Utilities|FlowControl|Delay (Math|Random|RandomFloatinRange 0.01 0.5))
    (bind _newtrack_0 (Timeline|AttackAnimation PlayFromStart)
      (:Update
        (Transformation|SetWorldLocation (Variables|Default|GetCArdBody) (Math|Vector|Lerp(Vector) (Transformation|GetWorldLocation (Variables|Default|GetDefaultSceneRoot)) (Transformation|GetWorldLocation (Variables|/Game/Blueprints/BP_GameCamera.BP_GameCamera_C|GetJunkLocation (Variables|Default|GetPlayerREf))) _newtrack_0) false false))
      (:Finished
        (bind _output_get (Variables|/Game/Blueprints/BP_GameCamera.BP_GameCamera_C|SetHP _playerref (- (Variables|/Game/Blueprints/BP_GameCamera.BP_GameCamera_C|GetHP _playerref) (* 5.0 (Utilities|Array|Length (Variables|Default|GetIcons))))))
        (if (<= _output_get 0.0)
          (bind _returnvalue (UserInterface|CreateWidget "/Game/UI/UI_loose.UI_loose_C"))
          (UserInterface|Viewport|AddtoViewport _returnvalue 0)
          (Input|SetInputModeUIOnly (Game|GetPlayerController 0) _returnvalue "DoNotLock" false))))))

(event Custom|ClickOther
  (if (Variables|Default|GetIsEnemyCard)
    ;[1 0 0] If you click on enemy card. Battle starts.
    (Default|StopBattle (Variables|/Game/UI/UI_GameMain.UI_GameMain_C|GetUI_FightBar (Variables|/Game/Blueprints/BP_GameCamera.BP_GameCamera_C|GetMainUIRef (Variables|Default|GetPlayerREf))) false)
    (Default|BeginBattle (Variables|/Game/UI/UI_GameMain.UI_GameMain_C|GetUI_FightBar (Variables|/Game/Blueprints/BP_GameCamera.BP_GameCamera_C|GetMainUIRef (Variables|Default|GetPlayerREf))) (Variables|Default|GetMyData) self)
    (else
      ;[1 1 1] If you hit ally card, you begin dragging or maybe show card to activate effects maybe.
      (Default|StopBattle (Variables|/Game/UI/UI_GameMain.UI_GameMain_C|GetUI_FightBar (Variables|/Game/Blueprints/BP_GameCamera.BP_GameCamera_C|GetMainUIRef (Variables|Default|GetPlayerREf))) false)
      (Variables|/Game/Blueprints/BP_GameCamera.BP_GameCamera_C|SetHoldPreview (Variables|Default|GetPlayerREf) true)
      (Utilities|FlowControl|Gate true) ; enters at Open
    )))

(event Custom|CardDestroyed
  (params (FromBattle :type Boolean))
  ;[1 1 1] When card is destroy. Make sure to destroy icons
  (for _array_element (Variables|Default|GetIcons)
    (Actor|DestroyActor _array_element))
  (Actor|DestroyActor))

(event Custom|CustomEffect
  (bind _playerref (Variables|Default|GetPlayerREf))
  (bind _cardsinarea (Variables|Default|GetCardsInArea))
  (Default|StopPreview (Variables|Default|GetPlayerREf))
  ;[1 1 1] InstantEffect
  (switch string (.name (Variables|Default|GetMyData))
    (:Goblin%20Assault
      (CallFunction|AddDomination 1000))
    (:Plundering
      (bind _icons (Default|GetAllWarIcons _playerref))
      (Variables|/Game/Blueprints/BP_GameCamera.BP_GameCamera_C|SetGold _playerref (+ (Variables|/Game/Blueprints/BP_GameCamera.BP_GameCamera_C|GetGold _playerref) (* 3 (Utilities|Array|Length _icons)))))
    (:Medic
      (Development|PrintString (Utilities|String|ToString(Integer) (Utilities|Array|Length _cardsinarea)))
      (for _array_element _cardsinarea
        (bind _asbp_card (Utilities|Casting|CastToBP_Card _array_element))
        (CallFunction|RestoreIcons _asbp_card false (Utilities|Array|MakeArray "NewEnumerator5" "NewEnumerator4"))))))

(event Custom|EndOfTurnEffect
  ;[1 0.1889 0] End of turn effects
  (Variables|Default|SetInitialLocation (Transformation|GetActorLocation))
  (bind _newtrack_0 (Timeline|DoJump PlayFromStart)
    (:Update
      (Transformation|SetActorLocation (Math|Vector|Lerp(Vector) (Variables|Default|GetInitialLocation) (+ (Variables|Default|GetInitialLocation) "0.000000,0.000000,5.000000") _newtrack_0) false false))))

(event Custom|AfterJumping
  ;[1 0.1889 0] End of turn effects
  (Audio|PlaySound2D "/Game/Sound/Au_Slamming_Cue.Au_Slamming_Cue" 1.0 0.05 0.0 0 0)
  ;;[1 1 1] EndTurnEffect
  (switch string (.name (Variables|Default|GetMyData))
    (:Troll%20Pit
      (CallFunction|AddDomination (* (Variables|/Game/Blueprints/BP_GameCamera.BP_GameCamera_C|GetFood (Variables|Default|GetPlayerREf)) 500)))
    (:Skeleton
      (bind _outactors (Actor|GetAllActorsOfClass "BP_Card_C"))
      (for _array_element _outactors
        (CallFunction|DeathEffect _array_element))
      (Utilities|FlowControl|Delay 0.69)
      (CallFunction|CardDestroyed false))
    (:The%20Dark%20Lord
      (bind _outactors_2 (Actor|GetAllActorsOfClass "/Game/Blueprints/BP_TapIcon.BP_TapIcon_C"))
      (for _array_element_2 _outactors_2
        (if (not (Variables|/Game/Blueprints/BP_TapIcon.BP_TapIcon_C|GetIsEnemy _array_element_2))
          (Utilities|SeeifWarorMagic _array_element_2
            (:True
              (CallFunction|AddDomination 500))))))))

(event Custom|ActiveEffect
  (switch string (.name (Variables|Default|GetMyData))
    (:Siege%20Master
      (bind _newparam (CallFunction|FindTagsforWarRestore "Troll"))
      (Utilities|IsValid (.OutItem (Utilities|Array|Random _newparam))
        (:Is%20Valid
          (CallFunction|RestoreIcons (.OutItem (Utilities|Array|Random _newparam)) false (Utilities|Array|MakeArray "NewEnumerator5")))
        (:Is%20Not%20Valid
          (Development|PrintString "No Target"))))
    (:Sword%20Master%20Goblin
      (CallFunction|RestoreIcons false (Utilities|Array|MakeArray "NewEnumerator5" "NewEnumerator5")))))

(event Custom|DeathEffect
  (bind _playerref (Variables|Default|GetPlayerREf))
  (bind _playerref_2 (Variables|Default|GetPlayerREf))
  (switch string (.name (Variables|Default|GetMyData))
    (:Bone%20Altar
      (bind _newparam (CallFunction|FindTags "BoneMusalium"))
      (Variables|/Game/Blueprints/BP_GameCamera.BP_GameCamera_C|SetGold _playerref_2 (+ (Variables|/Game/Blueprints/BP_GameCamera.BP_GameCamera_C|GetGold _playerref_2) (Math|Integer|SelectInt 10 5 (> (Utilities|Array|Length _newparam) 0)))))
    (:Bone%20Crypt
      (bind _newparam_2 (CallFunction|FindTags "BoneMusalium"))
      (Variables|/Game/Blueprints/BP_GameCamera.BP_GameCamera_C|SetDominationPoint _playerref (+ (Variables|/Game/Blueprints/BP_GameCamera.BP_GameCamera_C|GetDominationPoint _playerref) (Math|Integer|SelectInt 1000 500 (> (Utilities|Array|Length _newparam_2) 0)))))))

(event EventBeginPlay
  (bind _asbp_game_camera (Utilities|Casting|CastToBP_GameCamera (Game|Player|GetPlayerPawn 0)))
  (Variables|Default|SetPlayerREf _asbp_game_camera)
  ;[1 1 1] Register Data and Location.
  (Variables|Default|SetInitialLocation (Variables|/Script/Engine.SceneComponent|GetRelativeLocation (Variables|Default|GetCArdBody)))
  (bind _asui_card (Utilities|Casting|CastToUI_card (UserInterface|GetWidget (Variables|Default|GetWidget))))
  (Variables|/Game/UI/UI_card.UI_card_C|SetSkipAnimation _asui_card true)
  (Variables|/Game/UI/UI_card.UI_card_C|SetMyData _asui_card (Variables|Default|GetMyData))
  ;[1 1 1] Animate card flying onto the table
  (bind _newtrack_0 (Timeline|PlayOnBoard PlayFromStart)
    (:Update
      (Transformation|SetRelativeLocation (Variables|Default|GetCArdBody) (Math|Vector|Lerp(Vector) (Variables|Default|GetInitialLocation) "0, 0, 0" _newtrack_0) false false))
    (:Finished
      (Audio|PlaySound2D "/Game/Sound/Au_Slamming_Cue.Au_Slamming_Cue" 1.0 1.0 0.0 0 0)
      (CallFunction|OnPlayed))))

(event EventTick
  (params (DeltaSeconds :type Float%20%28single-precision%29))
  ;[1 1 1] If you hit ally card, you begin dragging or maybe show card to activate effects maybe.
  (Utilities|FlowControl|Gate true
    (:Exit
      (Transformation|SetActorLocation (.location (.HitResult (Class|PlayerController|GetHitResultUnderCursorforObjects (Game|GetPlayerController 0) (Utilities|Array|MakeArray "ObjectTypeQuery1") true))) false false))))

(fn ConstructionScript)

(fn AddDomination
  (params (AddPoints :type Integer))
  (bind _playerref (Variables|Default|GetPlayerREf))
  (bind _output_get (Variables|/Game/Blueprints/BP_GameCamera.BP_GameCamera_C|SetDominationPoint _playerref (+ (Variables|/Game/Blueprints/BP_GameCamera.BP_GameCamera_C|GetDominationPoint _playerref) AddPoints)))
  (return _output_get))

(fn ReorderIcons
  (bind _returnvalue (Transformation|GetActorLocation))
  (for (_array_element _array_index) (Variables|Default|GetIcons)
    (Transformation|SetActorLocation _array_element (Math|Vector|MakeVector (.x _returnvalue) (+ (.y _returnvalue) (* _array_index (Variables|Default|GetSpace)) (* (* (Variables|Default|GetSpace) 0.5 (- (Utilities|Array|Length (Variables|Default|GetIcons)) 1)) -1.0)) (.z _returnvalue)) false false)))

(fn FindTagsforWarRestore
  (params (tag :type String))
  (bind _outactors (Actor|GetAllActorsOfClass "BP_Card_C"))
  (for _array_element _outactors
    (if (not (== _array_element self))
      (if (Utilities|Array|ContainsItem (.tags (Variables|BP_Card_C|GetMyData _array_element)) tag)
        (if (> (Utilities|Array|Length (Variables|BP_Card_C|GetMissingIcons _array_element)) 0)
          (Utilities|Array|Add (LocalVariables|GetFoundCArds) _array_element)))))
  (return (LocalVariables|GetFoundCArds)))

(fn NewFunction
  (params (FullArray :type Array%20of%20enum_Resources%20Enums :default "NewEnumerator0") (RemoveList :type Array%20of%20enum_Resources%20Enums :default "NewEnumerator0")))

(fn FindTags
  (params (tag :type String))
  (bind _outactors (Actor|GetAllActorsOfClass "BP_Card_C"))
  (for _array_element _outactors
    (if (not (== _array_element self))
      (if (Utilities|Array|ContainsItem (.tags (Variables|BP_Card_C|GetMyData _array_element)) tag)
        (Utilities|Array|Add (LocalVariables|GetFoundCArds) _array_element))))
  (return (LocalVariables|GetFoundCArds)))